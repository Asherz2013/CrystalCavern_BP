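; BP_Cannon is an automatic cannon that fires projectiles repeatedly from the moment play begins.
; After each fire-rate delay it spawns a scaled BP_Projectile at the spawn point's world location and rotation, then plays the CannonFire timeline.
; The timeline animates the barrel along its local Y axis, and its completion restarts the delay, so the firing interval includes the animation's length.
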(event `self.ReceiveBeginPlay`
  (`KismetSystemLibrary.Delay` (`self.CannonFireRate`) :!label _label)
  (`self.SpawnProjectile`)
  (bind (_direction _barrellocation) (`Timeline|CannonFire` :!via `PlayFromStart`)
    (:`Update`
      (`self.MoveCannonBarrel` _barrellocation))
    (:`Finished`
      (goto _label))))

(fn `MoveCannonBarrel`
  (params (`Cannon Barrel Y Location` :type "Float (double-precision)"))
  (`SceneComponent.K2_SetRelativeLocation` (`self.CannonBarrel`) (`KismetMathLibrary.MakeVector` 0.0 `Cannon Barrel Y Location`) false false))

(fn `SpawnProjectile`
  (bind _projectilespawnpoint (`self.ProjectileSpawnPoint`))
  (`|SpawnActorFromClass` "/Game/Blueprints/Actors/Projectiles/BP_Projectile.BP_Projectile_C" (`KismetMathLibrary.MakeTransform` (`SceneComponent.K2_GetComponentLocation` _projectilespawnpoint) (`SceneComponent.K2_GetComponentRotation` _projectilespawnpoint) (`KismetMathLibrary.Conv_DoubleToVector` (`self.ProjecileScale`))) "Undefined" "OverrideRootScale" null null))

(fn `UserConstructionScript`)