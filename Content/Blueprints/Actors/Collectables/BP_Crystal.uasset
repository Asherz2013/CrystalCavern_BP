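; BP_Crystal is a collectable crystal with a point light that flies into the player and vanishes when the player overlaps it.
; On overlap, a player-pawn check passes, starting location, scale and light intensity are stored, and a collection timeline plays.
; Timeline curves drive lerps that home on the pawn's current location, shrink the crystal to zero and fade its light, then the actor is destroyed.
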(event `self.ReceiveActorBeginOverlap`
  (params (OtherActor :type "Actor Object Reference"))
  (`self.IsPlayer` OtherActor
    (:`IsPlayer`
      (`self.StoreStartingValues`)
      (bind (_direction _collectionprogress _scaleprogress _lightintensity) (`Timeline|CollectionTimeline`)
        (:`Update`
          (`self.MoveToActorLocation` _collectionprogress (`GameplayStatics.GetPlayerPawn` 0))
          (`self.ScaleCrystal` _scaleprogress)
          (`self.AdjustLight` _lightintensity))
        (:`Finished`
          (`self.K2_DestroyActor`))))))

(fn `AdjustLight`
  (params (Alpha :type "Float (double-precision)"))
  (`LightComponent.SetIntensity` (`self.PointLight`) (`KismetMathLibrary.Lerp` (`self.StartIntensity`) 0.0 Alpha)))

(fn `MoveToActorLocation`
  (params (Alpha :type "Float (double-precision)") (Actor :type "Actor Object Reference"))
  (`self.K2_SetActorLocation` (`KismetMathLibrary.VLerp` (`self.StartLocation`) (`self.K2_GetActorLocation` Actor) Alpha)))

(fn `ScaleCrystal`
  (params (Alpha :type "Float (double-precision)"))
  (`self.SetActorScale3D` (`KismetMathLibrary.VLerp` (`self.StartScale`) (0.0 0.0 0.0) Alpha)))

(fn `StoreStartingValues`
  (set `self.StartLocation` (`self.K2_GetActorLocation`))
  (set `self.StartScale` (`self.GetActorScale3D`))
  (set `self.StartIntensity` (`LightComponentBase.Intensity` (`self.PointLight`))))

(fn `UserConstructionScript`)